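; BP_VendingMachine is an interactable vending machine actor that opens a purchase-style UI widget.
; Overlap begin and end cast the other actor and show or hide the interact prompt text on that actor's PlayerHUD.
; The BPIInteraction interface event creates a W_VendingMachineUI widget and adds it to the viewport.
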(event Collision|EventActorBeginOverlap
  (params (OtherActor :type Actor%20Object%20Reference))
  (bind _asbp_character_base (Utilities|Casting|CastTo OtherActor))
  (Widget|SetVisibility (Variables|/Game/Pack/Aurora/UI/W_PlayerHUD.W_PlayerHUD_C|GetInteractPrompt_TXT (Variables|Default|GetPlayerHUD _asbp_character_base)) "Visible"))

(event Collision|EventActorEndOverlap
  (params (OtherActor :type Actor%20Object%20Reference))
  (bind _asbp_character_base (Utilities|Casting|CastTo OtherActor))
  (Widget|SetVisibility (Variables|/Game/Pack/Aurora/UI/W_PlayerHUD.W_PlayerHUD_C|GetInteractPrompt_TXT (Variables|Default|GetPlayerHUD _asbp_character_base)) "Hidden"))

(event EventBPIInteraction
  (bind _returnvalue (UserInterface|CreateWidget "/Game/Pack/Aurora/UI/W_VendingMachineUI.W_VendingMachineUI_C"))
  (UserInterface|Viewport|AddtoViewport _returnvalue 0))

(fn ConstructionScript)