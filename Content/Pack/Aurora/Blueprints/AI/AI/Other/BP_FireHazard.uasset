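; BP_FireHazard is a fire hazard actor that damages the player over time.
; It plays a sound at its location on BeginPlay.
; An overlap that passes a cast starts a looping half-second Damage timer, and the matching end overlap clears it.
; Each tick of that timer applies a small hit to player character 0, rather than to the stored overlapping actor, with the hazard as damage causer.
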(event Custom|Damage
  (Game|Damage|ApplyDamage (Game|GetPlayerCharacter 0) 0.1 0 self))

(event EventBeginPlay
  (Audio|PlaySoundatLocation 0 (Transformation|GetActorLocation)))

(event Collision|EventActorBeginOverlap
  (params (OtherActor :type Actor%20Object%20Reference))
  (Utilities|Casting|CastTo OtherActor)
  (Utilities|Time|SetTimerbyFunctionName 0 "Damage" 0.5 true))

(event Collision|EventActorEndOverlap
  (params (OtherActor :type Actor%20Object%20Reference))
  (Utilities|Casting|CastTo OtherActor)
  (Utilities|Time|ClearTimerbyFunctionName 0 "Damage"))

(fn ConstructionScript)