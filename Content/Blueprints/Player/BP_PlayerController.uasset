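; Player controller that handles respawning through the game mode.
; Pressing Enter while controlling a BP_GameSpectator sends a server respawn request, honored only if the game mode allows fast respawn.
; LaunchRespawnTimer schedules the same Respawn function after a given delay and stores the timer handle, without checking that flag.
; Respawn delegates the actual spawning to BP_BaseGamemode's SpawnPlayer.
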(event Custom|Server-Respawn
  (bind _asbp_base_gamemode (Utilities|Casting|CastToBP_BaseGamemode (Game|GetGameMode)))
  (if (Variables|/Game/Blueprints/Game/BP_BaseGamemode.BP_BaseGamemode_C|GetAllowFastRespawn _asbp_base_gamemode)
    (CallFunction|Respawn)))

(event Input|KeyboardEvents|Enter
  (params (Key :type Key%20Structure :default "AnyKey"))
  (:Pressed
    (Utilities|Casting|CastToBP_GameSpectator (Pawn|GetControlledPawn))
    (CallFunction|Server-Respawn)))

(fn ConstructionScript)

(fn Respawn
  (bind _asbp_base_gamemode (Utilities|Casting|CastToBP_BaseGamemode (Game|GetGameMode)))
  (Default|SpawnPlayer _asbp_base_gamemode self))

(fn LaunchRespawnTimer
  (params (Time :type Float%20%28single-precision%29))
  (bind _returnvalue (Utilities|Time|SetTimerbyFunctionName 0 "Respawn" Time))
  (Variables|Default|SetRespawnTimer _returnvalue))