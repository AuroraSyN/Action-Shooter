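; Rifle weapon Blueprint whose secondary action is a sniper-style scoped aim.
; Extending the parent's secondary action events, it zeroes spread while aiming and restores the class default on release.
; For the local player only, it narrows the camera FOV, shows a scope widget and plays placeholder animations, then resets FOV and removes the widget when aiming stops.
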(event EventUseSecondaryAction
  (|CallParentFunction)
  (if (Variables|Default|GetUsingSecondary)
    (Variables|Default|SetSpreadAngle 0.0)
    (if (Pawn|IsLocalPlayerController (Game|GetInstigatorController))
      (Camera|SetFieldOfView (Variables|/Game/Blueprints/Player/BP_PlayerCharacter.BP_PlayerCharacter_C|GetCamera (Variables|Default|GetWeaponOwner)) 55.0)
      (Variables|Default|GetSniperScope
        (:then
          _)
        (:else
          (UserInterface|CreateWidget "/Game/UI/Other/SniperScope/W_Scope.W_Scope_C")
          (bind _output_get (Variables|Default|SetSniperScope 0))))
      (UserInterface|Viewport|AddtoViewport _output_get -1)
      ;[1 1 1] Add your weapon animations here
      (Components|Animation|PlayAnimation (Variables|Default|GetSkeletalMesh) "/Game/Assets/Characters/Mannequin/Animations/Fire_Shotgun_Hip.Fire_Shotgun_Hip" true)
      (Components|Animation|PlayAnimation (Variables|Default|GetSkeletalMesh) "/Game/Assets/Characters/Mannequin/Animations/Aim_Space_Hip.Aim_Space_Hip" true))))

(event EventStopUseSecondaryAction
  (|CallParentFunction)
  (Variables|Default|SetSpreadAngle (Utilities|GetClassDefaults (Utilities|GetClass self)))
  (if (Pawn|IsLocalPlayerController (Game|GetInstigatorController))
    (Camera|SetFieldOfView (Variables|/Game/Blueprints/Player/BP_PlayerCharacter.BP_PlayerCharacter_C|GetCamera (Variables|Default|GetWeaponOwner)) 9e+01)
    (Widget|RemovefromParent (Variables|Default|GetSniperScope))))

(fn ConstructionScript
  (|CallParentFunction))