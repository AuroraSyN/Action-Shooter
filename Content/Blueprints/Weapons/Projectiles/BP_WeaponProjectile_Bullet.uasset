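; Bullet projectile for fire weapons that deals point damage and leaves bullet-hole decals on impact.
; On hit, the authority applies point damage, reports it to the owning weapon and destroys the projectile.
; Remote instances instead spawn a short-lived decal actor oriented to the hit normal, using the weapon's hole material.
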(event Collision|EventHit
  (params (MyComp :type Primitive%20Component%20Object%20Reference) (Other :type Actor%20Object%20Reference) (OtherComp :type Primitive%20Component%20Object%20Reference) (bSelfMoved :type Boolean) (HitLocation :type Vector :default "0, 0, 0") (HitNormal :type Vector :default "0, 0, 0") (NormalImpulse :type Vector :default "0, 0, 0") (Hit :type Hit%20Result%20Structure%20%28by%20ref%29))
  (bind (_bblockinghit _binitialoverlap _time _distance _location _impactpoint _normal _impactnormal _physmat _hitactor _hitcomponent _hitbonename _hititem _faceindex _tracestart _traceend) (Collision|BreakHitResult Hit))
  (Networking|SwitchHasAuthority
    (:Authority
      (bind _returnvalue (Game|Damage|ApplyPointDamage Other (Variables|Default|GetDamage) (Math|Vector|GetUnitDirection(Vector) _traceend _tracestart) Hit (Game|GetInstigatorController) (Components|GetOwner)))
      (Default|OnWeaponDamagedActor (Variables|Default|GetWeapon) _returnvalue Other)
      (Actor|DestroyActor))
    (:Remote
      (|SpawnDecal HitLocation HitNormal))))

(fn ConstructionScript
  (|CallParentFunction))