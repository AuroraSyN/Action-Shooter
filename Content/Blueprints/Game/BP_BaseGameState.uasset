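; Base game state that runs the round lifecycle: pre-start countdown, timed round, end and map vote.
; On the authority, a one-second Tick counts down once enough players join, starts the round through the game mode, then reports when the time limit is reached.
; Clients learn of round start through RepNotify and round end through multicast.
; Round end triggers a vote, then server travel to the winning data-table map.
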(event EventBeginPlay
  (Networking|SwitchHasAuthority
    (:Authority
      (|Bindroundend))))

(event EventTick
  (params (DeltaSeconds :type Float%20%28single-precision%29))
  (Networking|SwitchHasAuthority
    (:Authority
      (switch Utilities|FlowControl|Switch|SwitchonE_GameState (Variables|Default|GetRoundInProgress)
        (:NewEnumerator0
          (if (CallFunction|EnoughPlayerstoStartRound)
            (bind _result (Math|Integer|DecrementInt (Variables|Default|GetRoundStartTime))
              (:%20%20
                (if (<= _result 0)
                  (Default|StartRound (CallFunction|GetGamemode))
                  (Variables|Default|SetRoundInProgress "NewEnumerator1"))))
            (else
              (Variables|Default|SetRoundStartTime (.RoundStartTime (Utilities|GetClassDefaults (Utilities|GetClass self)))))))
        (:NewEnumerator1
          (CallFunction|RoundTimeTick))))))

(fn ConstructionScript)

(fn RoundTimeTick
  (bind _output_get (Variables|RoundTime|SetRoundTime (+ (Variables|RoundTime|GetRoundTime) (Math|Timespan|MakeTimespan 0 0 0 1)))) ; + 1 sec to round time
  (Variables|RoundTime|SetCurrentMinute (.Minutes (Math|Timespan|BreakTimespan _output_get)))
  (Variables|RoundTime|SetCurrentSecond (.Seconds (Math|Timespan|BreakTimespan _output_get)))
  (if (and (>= (Variables|RoundTime|GetRoundTime) (Variables|/Game/Blueprints/Game/BP_BaseGamemode.BP_BaseGamemode_C|GetTimeLimit (CallFunction|GetGamemode))) (Utilities|Enum|Equal(Enum) (Variables|Default|GetRoundInProgress) "NewEnumerator1")) ; Time limit reachd
    (Default|TimeLimitReched (CallFunction|GetGamemode))))

(fn GetRoudTime
  (return (Variables|RoundTime|GetCurrentMinute) (Variables|RoundTime|GetCurrentSecond)))

(fn OnRepRoundinProgress
  (switch Utilities|FlowControl|Switch|SwitchonE_GameState (Variables|Default|GetRoundInProgress)
    (:NewEnumerator1
      (Default|CallRoundStarted))))

(fn GetPreRoundTime
  (return (Variables|Default|GetRoundStartTime)))

(fn NewPlayerConnected
  (params (PlayerState :type BP%20Player%20State%20Object%20Reference))
  (CallFunction|PrintMessage (Utilities|String|Append "Player connected: " (Utilities|GetDisplayName PlayerState)) "(R=1.000000,G=0.899090,B=0.000000,A=1.000000)" 2.0 false)
  (Default|CallPlayerConnected PlayerState))

(fn EnoughPlayerstoStartRound
  (return (>= (Utilities|Array|Length (Variables|Default|GetPlayerArray)) (Variables|Default|GetMatchStartWithPlayers))))

(fn TravelServertoMap
  (params (Map :type Name))
  (Development|ExecuteConsoleCommand (Utilities|String|Append "ServerTravel " (Utilities|String|ToString(Name) Map))))

(event Custom|OnRoundStarted
  (Variables|Default|SetRoundInProgress "NewEnumerator0"))

(event Custom|OnRoundEnded
  (params (Reason :type String))
  (CallFunction|Multicast-RoundEnd Reason)
  (Variables|Default|SetRoundInProgress "NewEnumerator2")
  (Default|StartVote (Variables|Default|GetBP_MapVoteController))
  (EventDispatchers|AssignVoteEnded (Variables|Default|GetBP_MapVoteController) (delegate Custom|VoteEnded)))

(event Custom|Multicast-RoundEnd
  (params (Reason :type String))
  (Default|CallRoundEnded Reason))

(event Custom|VoteEnded
  (params (VotedMap :type Name))
  (bind _returnvalue (Utilities|GetDataTableRow "/Game/Data/DataTables/DT_VoteMaps.DT_VoteMaps" VotedMap)
    (:then
      (CallFunction|TravelServertoMap (.mapname _returnvalue)))))